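; MyAsistivnaBall is an actor with a camera that follows balls and passes player input to the UI.
; On BeginPlay it shows a MainWidget, and the Next and Back inputs set flags on that widget.
; Each Tick, PratiKameru trails the camera behind MyBullin actors, otherwise VratiKameru returns it behind MyAsistivnaBall actors.
; Camera X eases at constant speed to an offset, Y snaps to the target and height stays fixed.
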(event EventBeginPlay
  (bind _returnvalue (UserInterface|CreateWidget "/Game/Blueprints/widgets/MainWidget.MainWidget_C"))
  (UserInterface|Viewport|AddtoViewport _returnvalue 0))

(event Collision|EventActorBeginOverlap
  (params (OtherActor :type Actor%20Object%20Reference)))

(event EventTick
  (params (DeltaSeconds :type Float%20%28single-precision%29))
  (bind _camera (Variables|Default|GetCamera))
  (bind _camera_2 (Variables|Default|GetCamera))
  (if (Variables|Default|GetpratiKameru)
    (bind _outactors (Actor|GetAllActorsOfClass "/Game/Blueprints/MyBullin.MyBullin_C"))
    (for _array_element _outactors
      (Transformation|SetWorldLocation _camera_2 (Math|Vector|MakeVector (.x (Math|Interpolation|VInterptoConstant (Transformation|GetWorldLocation _camera_2) (Math|Vector|MakeVector (- (.x (Transformation|GetWorldLocation (Variables|/Script/Asistivna.Bullin|GetBullin _array_element))) 1.2e+03) (.y (Transformation|GetWorldLocation (Variables|/Script/Asistivna.Bullin|GetBullin _array_element))) (.z (Transformation|GetWorldLocation (Variables|/Script/Asistivna.Bullin|GetBullin _array_element)))) (Utilities|Time|GetWorldDeltaSeconds) 6e+02)) (.y (Transformation|GetWorldLocation (Variables|/Script/Asistivna.Bullin|GetBullin _array_element))) (.z (Transformation|GetWorldLocation _camera_2))) false false))
    (elif (Variables|Default|GetvratiKameru)
      (bind _outactors_2 (Actor|GetAllActorsOfClass "MyAsistivnaBall_C"))
      (for _array_element_2 _outactors_2
        (Transformation|SetWorldLocation _camera (Math|Vector|MakeVector (.x (Math|Interpolation|VInterptoConstant (Transformation|GetWorldLocation _camera) (Math|Vector|MakeVector (- (.x (Transformation|GetWorldLocation (Variables|/Script/Engine.Actor|GetRootComponent _array_element_2))) 8.5e+02) (.y (Transformation|GetWorldLocation (Variables|/Script/Engine.Actor|GetRootComponent _array_element_2))) (.z (Transformation|GetWorldLocation (Variables|/Script/Engine.Actor|GetRootComponent _array_element_2)))) (Utilities|Time|GetWorldDeltaSeconds) 6e+02)) (.y (Transformation|GetWorldLocation (Variables|/Script/Engine.Actor|GetRootComponent _array_element_2))) (.z (Transformation|GetWorldLocation _camera))) false false)))))

(event Input|ActionEvents|InputActionNext
  (params (Key :type Key%20Structure :default "None"))
  (:Pressed
    (Variables|/Game/Blueprints/widgets/MainWidget.MainWidget_C|SetPressed_Next (stale EventBeginPlay _returnvalue) true)))

(event Input|ActionEvents|InputActionBack
  (params (Key :type Key%20Structure :default "None"))
  (:Pressed
    (Variables|/Game/Blueprints/widgets/MainWidget.MainWidget_C|SetPressed_Back (stale EventBeginPlay _returnvalue) true)))

(fn ConstructionScript)