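; LineAngle is an aiming indicator actor that lets the player's AsistivnaBall pawn pick a line direction and throw angle.
; Each Tick, it shows the clock-hand component only during aiming phases, snapping to the ball's location.
; In bar phase 1 it spins in yaw and writes the pawn's LineVector.
; Past phase 3, until thrown, it swings roll between 0 and -90 degrees and writes ThrowVector.
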(event Custom|ThrowAngle
  (bind _defaultsceneroot (Variables|Default|GetDefaultSceneRoot))
  (bind _returnvalue (Transformation|GetWorldRotation _defaultsceneroot))
  (if (and (not (Variables|/Script/Asistivna.AsistivnaBall|GetthrowIt (stale EventBeginPlay _asasistivna_ball))) (> (Class|AsistivnaBall|GetBarFaze (stale EventBeginPlay _asasistivna_ball)) 3))
    (CallFunction|ChangeVerticalAngleSpeed)
    (Transformation|SetWorldRotation _defaultsceneroot (Math|Rotator|MakeRotator (+ (.roll _returnvalue) (Variables|Default|GetVerticalAngleSpeed)) (.pitch _returnvalue) (.yaw _returnvalue)) false false)
    (bind _asasistivna_ball (Utilities|Casting|CastToAsistivnaBall (Game|Player|GetPlayerPawn 0)))
    (Class|AsistivnaBall|SetThrowVector _asasistivna_ball (Math|Vector|RotateVector (Transformation|GetActorUpVector) "0.000000,180.000000,0.000000"))))

(event Custom|ChangeVerticalAngleSpeed
  (bind _defaultsceneroot (Variables|Default|GetDefaultSceneRoot))
  (bind _returnvalue (Transformation|GetWorldRotation _defaultsceneroot))
  (if (>= (.roll _returnvalue) 0.0)
    (Variables|Default|SetVerticalAngleSpeed -1.0)
    (elif (<= (.roll _returnvalue) -9e+01)
      (Variables|Default|SetVerticalAngleSpeed 1.0))))

(event Custom|LineAngle%20Rotation
  (params (DeltaSeconds :type Float%20%28single-precision%29))
  (bind _defaultsceneroot (Variables|Default|GetDefaultSceneRoot))
  (bind _returnvalue (Transformation|GetWorldRotation _defaultsceneroot))
  (if (== (Class|AsistivnaBall|GetBarFaze (stale EventBeginPlay _asasistivna_ball)) 1)
    (Transformation|SetWorldRotation _defaultsceneroot (Math|Rotator|MakeRotator 0.0 (.pitch _returnvalue) (+ (.yaw _returnvalue) (Math|Conversions|ToFloat(Integer) (* (Class|AsistivnaBall|GetLineAngleSpeed (stale EventBeginPlay _asasistivna_ball)) (Math|Conversions|ToInteger(Boolean) (== (Class|AsistivnaBall|GetBarFaze (stale EventBeginPlay _asasistivna_ball)) 1)))))) false false)
    (bind _asasistivna_ball (Utilities|Casting|CastToAsistivnaBall (Game|Player|GetPlayerPawn 0)))
    (Class|AsistivnaBall|SetLineVector _asasistivna_ball (Math|Vector|RotateVector (Transformation|GetActorForwardVector) "0,90.000000, 0"))))

(event Custom|Set%20LineAngle%20Location
  (params (DeltaSeconds :type Float%20%28single-precision%29))
  (Transformation|SetWorldLocation (Variables|Default|GetDefaultSceneRoot) (Transformation|GetWorldLocation (Variables|/Script/Asistivna.AsistivnaBall|GetBall (stale EventBeginPlay _asasistivna_ball))) false false))

(event Custom|Set%20LineAngle%20Visibility
  (params (DeltaSeconds :type Float%20%28single-precision%29))
  (Rendering|SetVisibility (Variables|Default|GetClock_Seconds_Hand) (or (and (> (Class|AsistivnaBall|GetBarFaze (stale EventBeginPlay _asasistivna_ball)) 3) (not (Variables|/Script/Asistivna.AsistivnaBall|GetthrowIt (stale EventBeginPlay _asasistivna_ball)))) (== (Class|AsistivnaBall|GetBarFaze (stale EventBeginPlay _asasistivna_ball)) 1)) false)
  (if (or (and (> (Class|AsistivnaBall|GetBarFaze (stale EventBeginPlay _asasistivna_ball)) 3) (not (Variables|/Script/Asistivna.AsistivnaBall|GetthrowIt (stale EventBeginPlay _asasistivna_ball)))) (== (Class|AsistivnaBall|GetBarFaze (stale EventBeginPlay _asasistivna_ball)) 1))
    (CallFunction|SetLineAngleLocation 0.0)
    (CallFunction|LineAngleRotation 0.0)
    (CallFunction|ThrowAngle)))

(event EventBeginPlay
  (bind _asasistivna_ball (Utilities|Casting|CastToAsistivnaBall (Game|Player|GetPlayerPawn 0))))

(event EventTick
  (params (DeltaSeconds :type Float%20%28single-precision%29))
  (CallFunction|SetLineAngleVisibility 0.0))

(fn ConstructionScript)